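; Player controller for a two-player Pong game, handling paddle input, game start, restart and the end-of-game menu.
; Keyboard and gamepad Enhanced Input actions move or charge the Paddle_Pawn of player controller 0 or 1.
; In the main menu, any key not in KeyNames starts the ball and switches to the score menu.
; FinishGame pauses behind PauseMenu; RestartController resets both paddles and destroys power-ups.
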(event Custom|RestartController
  (bind _aspaddle_pawn (Utilities|Casting|CastToPaddle_Pawn (Pawn|GetControlledPawn (Game|GetPlayerController 0))))
  (Default|RestartPaddle _aspaddle_pawn 9e+02)
  (Default|SetPawnDefaultRotation _aspaddle_pawn 2e+01 1.8e+02)
  (bind _aspaddle_pawn_2 (Utilities|Casting|CastToPaddle_Pawn (Pawn|GetControlledPawn (Game|GetPlayerController 1))))
  (Default|RestartPaddle _aspaddle_pawn_2 -9e+02)
  (Default|SetPawnDefaultRotation _aspaddle_pawn_2 2e+01 0.0)
  (bind _outactors (Actor|GetAllActorsOfClass "/Game/Blueprints/PowerUp.PowerUp_C"))
  (for _array_element _outactors
    (if (Utilities|IsValid _array_element)
      (Actor|DestroyActor _array_element))))

(event Custom|Finish%20Game
  (bind _self self)
  (bind _returnvalue (UserInterface|CreateWidget "/Game/Blueprints/Menus/PauseMenu.PauseMenu_C"))
  (UserInterface|Viewport|AddtoViewport _returnvalue 0)
  (Variables|Default|SetbShowMouseCursor _self true)
  (Input|SetInputModeUIOnly _self (Variables|/Game/Blueprints/Menus/PauseMenu.PauseMenu_C|GetRestart_Button _returnvalue) "DoNotLock" false)
  (Game|SetGamePaused true))

(event Input|EnhancedActionEvents|EnhancedInputActionIA_MoveKB0
  (params (ActionValue :type Vector%202D%20Structure) (ElapsedSeconds :type Float%20%28double-precision%29) (TriggeredSeconds :type Float%20%28double-precision%29) (InputAction :type Input%20Action%20Object%20Reference :default "/Game/Blueprints/EnhancedInputActions/IA_MoveKB0.IA_MoveKB0"))
  ;[1 1 1] Player 1
  (bind _aspaddle_pawn (Utilities|Casting|CastToPaddle_Pawn (Pawn|GetControlledPawn (Game|GetPlayerController 0))))
  (Default|MovePaddle _aspaddle_pawn (Math|Conversions|ToVector(Vector2D) ActionValue)))

(event Input|EnhancedActionEvents|EnhancedInputActionIA_Restart
  (params (ActionValue :type Boolean) (ElapsedSeconds :type Float%20%28double-precision%29) (TriggeredSeconds :type Float%20%28double-precision%29) (InputAction :type Input%20Action%20Object%20Reference :default "/Game/Blueprints/EnhancedInputActions/IA_Restart.IA_Restart"))
  (bind _asbp_gamemode (Utilities|Casting|CastToBP_Gamemode (Game|GetGameMode)))
  (Default|RestartGame _asbp_gamemode))

(event Input|EnhancedActionEvents|EnhancedInputActionIA_ChargeGP0
  (params (ActionValue :type Boolean) (ElapsedSeconds :type Float%20%28double-precision%29) (TriggeredSeconds :type Float%20%28double-precision%29) (InputAction :type Input%20Action%20Object%20Reference :default "/Game/Blueprints/EnhancedInputActions/IA_ChargeGP0.IA_ChargeGP0"))
  ;[1 1 1] Charge Player1
  (:Triggered
    (bind _aspaddle_pawn (Utilities|Casting|CastToPaddle_Pawn (Pawn|GetControlledPawn (Game|GetPlayerController 0))))
    (Default|ChargePaddle _aspaddle_pawn TriggeredSeconds))
  (:Completed
    (Default|StopPaddleCharge _aspaddle_pawn 2e+01 1.8e+02)))

(event Input|EnhancedActionEvents|EnhancedInputActionIA_ChargeKB1
  (params (ActionValue :type Boolean) (ElapsedSeconds :type Float%20%28double-precision%29) (TriggeredSeconds :type Float%20%28double-precision%29) (InputAction :type Input%20Action%20Object%20Reference :default "/Game/Blueprints/EnhancedInputActions/IA_ChargeKB1.IA_ChargeKB1"))
  ;[1 1 1] Charge Player2
  (:Triggered
    (bind _aspaddle_pawn (Utilities|Casting|CastToPaddle_Pawn (Pawn|GetControlledPawn (Game|GetPlayerController 1))))
    (Default|ChargePaddle _aspaddle_pawn TriggeredSeconds))
  (:Completed
    (Default|StopPaddleCharge _aspaddle_pawn 2e+01 0.0)))

(event Input|EnhancedActionEvents|EnhancedInputActionIA_ChargeKP1
  (params (ActionValue :type Boolean) (ElapsedSeconds :type Float%20%28double-precision%29) (TriggeredSeconds :type Float%20%28double-precision%29) (InputAction :type Input%20Action%20Object%20Reference :default "/Game/Blueprints/EnhancedInputActions/IA_ChargeKP1.IA_ChargeKP1"))
  ;[1 1 1] Charge Player2
  (:Triggered
    (bind _aspaddle_pawn (Utilities|Casting|CastToPaddle_Pawn (Pawn|GetControlledPawn (Game|GetPlayerController 1))))
    (Default|ChargePaddle _aspaddle_pawn TriggeredSeconds))
  (:Completed
    (Default|StopPaddleCharge _aspaddle_pawn 2e+01 0.0)))

(event Input|EnhancedActionEvents|EnhancedInputActionIA_MoveKB1
  (params (ActionValue :type Vector%202D%20Structure) (ElapsedSeconds :type Float%20%28double-precision%29) (TriggeredSeconds :type Float%20%28double-precision%29) (InputAction :type Input%20Action%20Object%20Reference :default "/Game/Blueprints/EnhancedInputActions/IA_MoveKB1.IA_MoveKB1"))
  ;[1 1 1] Player 2
  (bind _aspaddle_pawn (Utilities|Casting|CastToPaddle_Pawn (Pawn|GetControlledPawn (Game|GetPlayerController 1))))
  (Default|MovePaddle _aspaddle_pawn (Math|Conversions|ToVector(Vector2D) ActionValue)))

(event Input|EnhancedActionEvents|EnhancedInputActionIA_MoveGP1
  (params (ActionValue :type Vector%202D%20Structure) (ElapsedSeconds :type Float%20%28double-precision%29) (TriggeredSeconds :type Float%20%28double-precision%29) (InputAction :type Input%20Action%20Object%20Reference :default "/Game/Blueprints/EnhancedInputActions/IA_MoveGP1.IA_MoveGP1"))
  ;[1 1 1] Player 2
  (bind _aspaddle_pawn (Utilities|Casting|CastToPaddle_Pawn (Pawn|GetControlledPawn (Game|GetPlayerController 1))))
  (Default|MovePaddle _aspaddle_pawn (Math|Conversions|ToVector(Vector2D) ActionValue)))

(event Input|EnhancedActionEvents|EnhancedInputActionIA_MoveGP0
  (params (ActionValue :type Vector%202D%20Structure) (ElapsedSeconds :type Float%20%28double-precision%29) (TriggeredSeconds :type Float%20%28double-precision%29) (InputAction :type Input%20Action%20Object%20Reference :default "/Game/Blueprints/EnhancedInputActions/IA_MoveGP0.IA_MoveGP0"))
  ;[1 1 1] Player 1
  (bind _aspaddle_pawn (Utilities|Casting|CastToPaddle_Pawn (Pawn|GetControlledPawn (Game|GetPlayerController 0))))
  (Default|MovePaddle _aspaddle_pawn (Math|Conversions|ToVector(Vector2D) ActionValue)))

(event Input|EnhancedActionEvents|EnhancedInputActionIA_ChargeKB0
  (params (ActionValue :type Boolean) (ElapsedSeconds :type Float%20%28double-precision%29) (TriggeredSeconds :type Float%20%28double-precision%29) (InputAction :type Input%20Action%20Object%20Reference :default "/Game/Blueprints/EnhancedInputActions/IA_ChargeKB0.IA_ChargeKB0"))
  ;[1 1 1] Charge Player1
  (:Triggered
    (bind _aspaddle_pawn (Utilities|Casting|CastToPaddle_Pawn (Pawn|GetControlledPawn (Game|GetPlayerController 0))))
    (Default|ChargePaddle _aspaddle_pawn TriggeredSeconds))
  (:Completed
    (Default|StopPaddleCharge _aspaddle_pawn 2e+01 1.8e+02)))

(event Input|KeyboardEvents|AnyKey
  (params (Key :type Key%20Structure :default "None"))
  ;[1 1 1] Start Game
  (:Pressed
    (if (Variables|Default|GetIsInMainMenu?)
      (for _array_element (Variables|Default|GetKeyNames)
        (bind _output_get (Variables|Default|SetStart? (or (Variables|Default|GetStart?) (Utilities|Enum|Equal(Enum) _array_element (Class|KismetInputLibrary|KeyGetDisplayName Key false))))))
      (if _output_get
        _
        (else
          (bind _asbp_gamemode (Utilities|Casting|CastToBP_Gamemode (Game|GetGameMode)))
          (Default|ChangetoScoreMenu _asbp_gamemode)
          (Variables|Default|SetIsInMainMenu? false)
          (bind _returnvalue (Actor|GetActorOfClass "/Game/Blueprints/Pong_Ball.Pong_Ball_C"))
          (Variables|/Game/Blueprints/Pong_Ball.Pong_Ball_C|SetGameStarted _returnvalue true)))
      (Variables|Default|SetStart? false))))

(fn ConstructionScript)