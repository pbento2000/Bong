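; Game mode for a two-player local Pong game that runs match setup, scoring and the menu flow.
; On BeginPlay it shows the main menu, spawns the ball, and creates a player, possessed paddle and paddle lights per PlayerStart, with Enhanced Input mapping.
; AddScore ends the match through the controller at five points, otherwise notifies both paddles; AddPower forwards power to a player's paddle.
; Menu events swap widgets, and returning to main resets scores and ball.
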(event Custom|AddPower
  (params (LastPlayerHit :type Integer) (Float :type Float%20%28double-precision%29))
  (bind _playersinfo (Variables|Default|GetPlayersInfo))
  (if (== LastPlayerHit 1)
    (Default|AddPower (.player1pawn _playersinfo) Float)
    (else
      (Default|AddPower (.player2pawn _playersinfo) Float))))

(event Custom|RestartGame
  (bind _universalcontroller (Variables|Default|GetUniversalController))
  (Variables|Default|SetPlayer1Score 0)
  (Variables|Default|SetPlayer2Score 0)
  (bind _returnvalue (Actor|GetActorOfClass "/Game/Blueprints/Pong_Ball.Pong_Ball_C"))
  (if (Utilities|IsValid _returnvalue)
    (Default|SelfDestroy _returnvalue))
  (Default|RestartController _universalcontroller)
  (Variables|/Game/Blueprints/Pong_Controller.Pong_Controller_C|SetIsInMainMenu? _universalcontroller true)
  (Game|SpawnActorfromClass "/Game/Blueprints/Pong_Ball.Pong_Ball_C" (Math|Transform|MakeTransform "0, 0, 0" "0, 0, 0" "1.000000,1.000000,1.000000") "Undefined" "MultiplyWithRoot" 0 false 0))

(event Custom|ChangeToScoreMenu
  (Widget|RemovefromParent (Variables|Default|GetMainMenu))
  (Utilities|IsValid (Variables|Default|GetScoreMenu)
    (:Is%20Valid
      _)
    (:Is%20Not%20Valid
      (bind _returnvalue (UserInterface|CreateWidget "/Game/Blueprints/Menus/ScoreMenu.ScoreMenu_C"))
      (Variables|Default|SetScoreMenu _returnvalue)))
  (UserInterface|Viewport|AddtoViewport (Variables|Default|GetScoreMenu) 0))

(event Custom|ChangeToMainMenu
  (Widget|RemovefromParent (Variables|Default|GetScoreMenu))
  (UserInterface|Viewport|AddtoViewport (Variables|Default|GetMainMenu) 0)
  (CallFunction|RestartGame))

(event EventBeginPlay
  (bind _returnvalue (Game|GetPlayerController 0))
  ;[1 1 1] Spawn Players
  (Audio|PlaySound2D "/Game/Sounds/Soundtrack.Soundtrack" 1.0 1.0 0.0 0 0)
  (bind _returnvalue_2 (UserInterface|CreateWidget "/Game/Blueprints/Menus/MainMenu.MainMenu_C"))
  (UserInterface|Viewport|AddtoViewport _returnvalue_2 0)
  (Variables|Default|SetMainMenu _returnvalue_2)
  (Game|SpawnActorfromClass "/Game/Blueprints/Pong_Ball.Pong_Ball_C" (Math|Transform|MakeTransform "0, 0, 0" "0, 0, 0" "1.000000,1.000000,1.000000") "Undefined" "MultiplyWithRoot" 0 false 0)
  (bind _outactors (Actor|GetAllActorsOfClass "/Script/Engine.PlayerStart"))
  (for (_array_element _array_index) _outactors
    (Variables|Default|SetArray%20Index _array_index)
    (bind _returnvalue_3 (Class|GameplayStatics|CreatePlayer -1))
    (if (> (Variables|Default|GetArray%20Index) 0)
      (Input|AddMappingContext (PlayerController|LocalPlayerSubsystems|GetEnhancedInputLocalPlayerSubsystem _returnvalue_3) "/Game/Blueprints/EnhancedInputActions/IMC_Movement.IMC_Movement" 0 "(bIgnoreAllPressedKeysUntilRelease=True,bForceImmediately=False,bNotifyUserSettings=False)")
      (bind _returnvalue_4 (Game|SpawnActorfromClass "/Game/Blueprints/Paddle_Pawn.Paddle_Pawn_C" (Transformation|GetActorTransform _array_element) "Undefined" "MultiplyWithRoot" 0 1 0))
      (Pawn|Possess (Game|GetPlayerController 1) _returnvalue_4)
      (bind _returnvalue_5 (Game|SpawnActorfromClass "/Game/Blueprints/PaddleLights.PaddleLights_C" (Math|Transform|MakeTransform "-875.000000,0.000000,0.000000" "0, 0, 0" "1.000000,1.000000,1.000000") "Undefined" "MultiplyWithRoot" 0 0))
      (Variables|/Game/Blueprints/PaddleLights.PaddleLights_C|SetAssignedPaddle _returnvalue_5 _returnvalue_4)
      (Utilities|Struct|SetmembersinGamemode_PlayersInfo (Variables|Default|GetPlayersInfo) (stale _returnvalue_6) _returnvalue_4)
      (else
        (bind _aspong_controller (Utilities|Casting|CastToPong_Controller _returnvalue))
        (Input|AddMappingContext (PlayerController|LocalPlayerSubsystems|GetEnhancedInputLocalPlayerSubsystem _aspong_controller) "/Game/Blueprints/EnhancedInputActions/IMC_Movement.IMC_Movement" 0 "(bIgnoreAllPressedKeysUntilRelease=True,bForceImmediately=False,bNotifyUserSettings=False)")
        (bind _returnvalue_6 (Game|SpawnActorfromClass "/Game/Blueprints/Paddle_Pawn.Paddle_Pawn_C" (Transformation|GetActorTransform _array_element) "Undefined" "MultiplyWithRoot" 0 0 0))
        (Pawn|Possess _aspong_controller _returnvalue_6)
        (bind _returnvalue_7 (Game|SpawnActorfromClass "/Game/Blueprints/PaddleLights.PaddleLights_C" (Math|Transform|MakeTransform "875.000000,0.000000,0.000000" "0, 0, 0" "1.000000,1.000000,1.000000") "Undefined" "MultiplyWithRoot" 0 0))
        (Variables|/Game/Blueprints/PaddleLights.PaddleLights_C|SetAssignedPaddle _returnvalue_7 _returnvalue_6)
        (bind _aspong_controller_2 (Utilities|Casting|CastToPong_Controller _returnvalue))
        (Variables|Default|SetUniversalController _aspong_controller_2)))))

(fn ConstructionScript)

(fn AddScore
  (params (Player :type Integer))
  (bind _playersinfo (Variables|Default|GetPlayersInfo))
  (bind _playersinfo_2 (Variables|Default|GetPlayersInfo))
  (if (== Player 1)
    (bind _result (Math|Integer|IncrementInt (Variables|Default|GetPlayer1Score))
      (:%20%20
        (bind _output_get (Variables|Default|SetPlayer1Score _result))
        (if (== _output_get 5)
          (Default|FinishGame (Variables|Default|GetUniversalController))
          (return true)
          (else
            (Default|PointScored (.player1pawn _playersinfo))
            (Default|PointScored (.player2pawn _playersinfo))
            (return false)))))
    (else
      (bind _result_2 (Math|Integer|IncrementInt (Variables|Default|GetPlayer2Score))
        (:%20%20
          (bind _output_get_2 (Variables|Default|SetPlayer2Score _result_2))
          (if (== _output_get_2 5)
            (Default|FinishGame (Variables|Default|GetUniversalController))
            (return true)
            (else
              (Default|PointScored (.player1pawn _playersinfo_2))
              (Default|PointScored (.player2pawn _playersinfo_2))
              (return false))))))))