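; BP_InputReceiver is a pawn handling keyboard and gamepad input for a two-player local paddle game.
; BeginPlay adds the mapping context and sets facing; most actions route to controller 0's or 1's pawn by action.
; Holding charge pitches the paddle and builds SpeedModifier, which feeds a movement debuff, while a Y-position check gates movement.
; PointScored banks the charge to offset continued holding; restart resets both Paddle_Pawns.
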(event Custom|PointScored
  (Variables|Default|SetLastRoundSpeedModifier (Variables|Default|GetSpeedModifier))
  (Variables|Default|SetSpeedModifier 0.0))

(event Custom|SetPawnDefaultRotation
  (params (Y%20Rot :type Float%20%28double-precision%29) (Z%20Rot :type Float%20%28double-precision%29))
  (Transformation|SetActorRotation (Math|Rotator|MakeRotator 0.0 Y%20Rot Z%20Rot)))

(event Input|EnhancedActionEvents|EnhancedInputActionIA_Restart
  (params (ActionValue :type Boolean) (ElapsedSeconds :type Float%20%28double-precision%29) (TriggeredSeconds :type Float%20%28double-precision%29) (InputAction :type Input%20Action%20Object%20Reference :default "/Game/Blueprints/EnhancedInputActions/IA_Restart.IA_Restart"))
  (:Triggered
    (Development|PrintString "Hello" :!label _label)
    (bind _aspaddle_pawn (Utilities|Casting|CastToPaddle_Pawn (Pawn|GetControlledPawn (Game|GetPlayerController 0))))
    (Default|RestartGame _aspaddle_pawn 0.0)
    (Default|SetPawnDefaultRotation _aspaddle_pawn 2e+01 1.8e+02)
    (bind _aspaddle_pawn_2 (Utilities|Casting|CastToPaddle_Pawn (Pawn|GetControlledPawn (Game|GetPlayerController 1))))
    (Default|RestartGame _aspaddle_pawn_2 0.0)
    (Default|SetPawnDefaultRotation _aspaddle_pawn_2 2e+01 0.0))
  (:Started
    (goto _label)))

(event Input|EnhancedActionEvents|EnhancedInputActionIA_MoveKB0
  (params (ActionValue :type Vector%202D%20Structure) (ElapsedSeconds :type Float%20%28double-precision%29) (TriggeredSeconds :type Float%20%28double-precision%29) (InputAction :type Input%20Action%20Object%20Reference :default "/Game/Blueprints/EnhancedInputActions/IA_MoveKB0.IA_MoveKB0"))
  ;[1 1 1] Movement P1
  (bind _asbp_input_receiver (Utilities|Casting|CastToBP_InputReceiver (Pawn|GetControlledPawn (Game|GetPlayerController 0))))
  (bind _returnvalue (Class|LogicandMaths|ApplyChargeDebuff (Variables|BP_InputReceiver_C|GetSpeedModifier _asbp_input_receiver) (Variables|BP_InputReceiver_C|GetLastRoundSpeedModifier _asbp_input_receiver) 1e+01))
  (bind _returnvalue_2 (Class|LogicandMaths|PlayerMovementCheckup ActionValue (.y (Transformation|GetActorLocation _asbp_input_receiver))))
  (if _returnvalue_2
    (Pawn|Input|AddMovementInput _asbp_input_receiver (Math|Conversions|ToVector(Vector2D) (* ActionValue (- 0.5 _returnvalue))) 1.0 false)))

(event Input|EnhancedActionEvents|EnhancedInputActionIA_ChargeGP0
  (params (ActionValue :type Boolean) (ElapsedSeconds :type Float%20%28double-precision%29) (TriggeredSeconds :type Float%20%28double-precision%29) (InputAction :type Input%20Action%20Object%20Reference :default "/Game/Blueprints/EnhancedInputActions/IA_ChargeGP0.IA_ChargeGP0"))
  (:Triggered
    (bind _asbp_input_receiver (Utilities|Casting|CastToBP_InputReceiver (Pawn|GetControlledPawn (Game|GetPlayerController 0))))
    (Transformation|AddActorLocalRotation _asbp_input_receiver (Math|Rotator|MakeRotator 0.0 TriggeredSeconds 0.0) false false)
    (Variables|BP_InputReceiver_C|SetSpeedModifier _asbp_input_receiver (- (* TriggeredSeconds 0.01) (Variables|Default|GetLastRoundSpeedModifier))))
  (:Completed
    (Variables|BP_InputReceiver_C|SetLastRoundSpeedModifier _asbp_input_receiver 0.0)
    (Variables|BP_InputReceiver_C|SetSpeedModifier _asbp_input_receiver 0.0)
    (CallFunction|SetPawnDefaultRotation _asbp_input_receiver 2e+01 1.8e+02)))

(event Input|EnhancedActionEvents|EnhancedInputActionIA_ChargeKB0
  (params (ActionValue :type Boolean) (ElapsedSeconds :type Float%20%28double-precision%29) (TriggeredSeconds :type Float%20%28double-precision%29) (InputAction :type Input%20Action%20Object%20Reference :default "/Game/Blueprints/EnhancedInputActions/IA_ChargeKB0.IA_ChargeKB0"))
  (:Triggered
    (bind _asbp_input_receiver (Utilities|Casting|CastToBP_InputReceiver (Pawn|GetControlledPawn (Game|GetPlayerController 0))))
    (Transformation|AddActorLocalRotation _asbp_input_receiver (Math|Rotator|MakeRotator 0.0 TriggeredSeconds 0.0) false false)
    (Variables|BP_InputReceiver_C|SetSpeedModifier _asbp_input_receiver (- (* TriggeredSeconds 0.01) (Variables|Default|GetLastRoundSpeedModifier))))
  (:Completed
    (Variables|BP_InputReceiver_C|SetLastRoundSpeedModifier _asbp_input_receiver 0.0)
    (Variables|BP_InputReceiver_C|SetSpeedModifier _asbp_input_receiver 0.0)
    (CallFunction|SetPawnDefaultRotation _asbp_input_receiver 2e+01 1.8e+02)))

(event Input|EnhancedActionEvents|EnhancedInputActionIA_MoveKB1
  (params (ActionValue :type Vector%202D%20Structure) (ElapsedSeconds :type Float%20%28double-precision%29) (TriggeredSeconds :type Float%20%28double-precision%29) (InputAction :type Input%20Action%20Object%20Reference :default "/Game/Blueprints/EnhancedInputActions/IA_MoveKB1.IA_MoveKB1"))
  ;[1 1 1] Movement P2
  (bind _asbp_input_receiver (Utilities|Casting|CastToBP_InputReceiver (Pawn|GetControlledPawn (Game|GetPlayerController 1))))
  (bind _returnvalue (Class|LogicandMaths|ApplyChargeDebuff (Variables|BP_InputReceiver_C|GetSpeedModifier _asbp_input_receiver) (Variables|BP_InputReceiver_C|GetLastRoundSpeedModifier _asbp_input_receiver) 1e+01))
  (bind _returnvalue_2 (Class|LogicandMaths|PlayerMovementCheckup ActionValue (.y (Transformation|GetActorLocation _asbp_input_receiver))))
  (if _returnvalue_2
    (Pawn|Input|AddMovementInput _asbp_input_receiver (Math|Conversions|ToVector(Vector2D) (* ActionValue (- 0.5 _returnvalue))) 1.0 false)))

(event Input|EnhancedActionEvents|EnhancedInputActionIA_MoveGP1
  (params (ActionValue :type Vector%202D%20Structure) (ElapsedSeconds :type Float%20%28double-precision%29) (TriggeredSeconds :type Float%20%28double-precision%29) (InputAction :type Input%20Action%20Object%20Reference :default "/Game/Blueprints/EnhancedInputActions/IA_MoveGP1.IA_MoveGP1"))
  ;[1 1 1] Movement P2
  (bind _asbp_input_receiver (Utilities|Casting|CastToBP_InputReceiver (Pawn|GetControlledPawn (Game|GetPlayerController 1))))
  (bind _returnvalue (Class|LogicandMaths|ApplyChargeDebuff (Variables|BP_InputReceiver_C|GetSpeedModifier _asbp_input_receiver) (Variables|BP_InputReceiver_C|GetLastRoundSpeedModifier _asbp_input_receiver) 1e+01))
  (bind _returnvalue_2 (Class|LogicandMaths|PlayerMovementCheckup ActionValue (.y (Transformation|GetActorLocation _asbp_input_receiver))))
  (if _returnvalue_2
    (Pawn|Input|AddMovementInput _asbp_input_receiver (Math|Conversions|ToVector(Vector2D) (* (Class|KismetMathLibrary|NormalSafe2D ActionValue 0.0) (- 0.5 _returnvalue))) 1.0 false)))

(event Input|EnhancedActionEvents|EnhancedInputActionIA_ChargeKB1
  (params (ActionValue :type Boolean) (ElapsedSeconds :type Float%20%28double-precision%29) (TriggeredSeconds :type Float%20%28double-precision%29) (InputAction :type Input%20Action%20Object%20Reference :default "/Game/Blueprints/EnhancedInputActions/IA_ChargeKB1.IA_ChargeKB1"))
  (:Triggered
    (Development|PrintString (Utilities|GetDisplayName self))
    (bind _asbp_input_receiver (Utilities|Casting|CastToBP_InputReceiver (Pawn|GetControlledPawn (Game|GetPlayerController 1))))
    (Transformation|AddActorLocalRotation _asbp_input_receiver (Math|Rotator|MakeRotator 0.0 TriggeredSeconds 0.0) false false)
    (Variables|BP_InputReceiver_C|SetSpeedModifier _asbp_input_receiver (- (* TriggeredSeconds 0.01) (Variables|Default|GetLastRoundSpeedModifier))))
  (:Completed
    (Variables|BP_InputReceiver_C|SetLastRoundSpeedModifier _asbp_input_receiver 0.0)
    (Variables|BP_InputReceiver_C|SetSpeedModifier _asbp_input_receiver 0.0)
    (CallFunction|SetPawnDefaultRotation _asbp_input_receiver 2e+01 0.0)))

(event Input|EnhancedActionEvents|EnhancedInputActionIA_ChargeKP1
  (params (ActionValue :type Boolean) (ElapsedSeconds :type Float%20%28double-precision%29) (TriggeredSeconds :type Float%20%28double-precision%29) (InputAction :type Input%20Action%20Object%20Reference :default "/Game/Blueprints/EnhancedInputActions/IA_ChargeKP1.IA_ChargeKP1"))
  (:Triggered
    (bind _asbp_input_receiver (Utilities|Casting|CastToBP_InputReceiver (Pawn|GetControlledPawn (Game|GetPlayerController 1))))
    (Transformation|AddActorLocalRotation _asbp_input_receiver (Math|Rotator|MakeRotator 0.0 TriggeredSeconds 0.0) false false)
    (Variables|BP_InputReceiver_C|SetSpeedModifier _asbp_input_receiver (- (* TriggeredSeconds 0.01) (Variables|Default|GetLastRoundSpeedModifier))))
  (:Completed
    (Variables|BP_InputReceiver_C|SetLastRoundSpeedModifier _asbp_input_receiver 0.0)
    (Variables|BP_InputReceiver_C|SetSpeedModifier _asbp_input_receiver 0.0)
    (CallFunction|SetPawnDefaultRotation _asbp_input_receiver 2e+01 0.0)))

(event Input|EnhancedActionEvents|EnhancedInputActionIA_MoveGP0
  (params (ActionValue :type Vector%202D%20Structure) (ElapsedSeconds :type Float%20%28double-precision%29) (TriggeredSeconds :type Float%20%28double-precision%29) (InputAction :type Input%20Action%20Object%20Reference :default "/Game/Blueprints/EnhancedInputActions/IA_MoveGP0.IA_MoveGP0"))
  ;[1 1 1] Movement P1
  (bind _asbp_input_receiver (Utilities|Casting|CastToBP_InputReceiver (Pawn|GetControlledPawn (Game|GetPlayerController 0))))
  (bind _returnvalue (Class|LogicandMaths|ApplyChargeDebuff (Variables|BP_InputReceiver_C|GetSpeedModifier _asbp_input_receiver) (Variables|BP_InputReceiver_C|GetLastRoundSpeedModifier _asbp_input_receiver) 1e+01))
  (bind _returnvalue_2 (Class|LogicandMaths|PlayerMovementCheckup ActionValue (.y (Transformation|GetActorLocation _asbp_input_receiver))))
  (if _returnvalue_2
    (Pawn|Input|AddMovementInput (Math|Conversions|ToVector(Vector2D) (* (Class|KismetMathLibrary|NormalSafe2D ActionValue 0.0) (- 0.5 _returnvalue))) 1.0 false)))

(event EventBeginPlay
  (Input|AddMappingContext (PlayerController|LocalPlayerSubsystems|GetEnhancedInputLocalPlayerSubsystem (Game|GetPlayerController (Variables|Default|GetPlayerIndex))) "/Game/Blueprints/EnhancedInputActions/IMC_Movement.IMC_Movement" 0 "(bIgnoreAllPressedKeysUntilRelease=True,bForceImmediately=False,bNotifyUserSettings=False)")
  (if (== (Variables|Default|GetPlayerIndex) 0)
    (bind _asbp_gamemode (Utilities|Casting|CastToBP_Gamemode (Game|GetGameMode)))
    (Utilities|Struct|SetmembersinGamemode_PlayersInfo (Variables|/Game/Blueprints/BP_Gamemode.BP_Gamemode_C|GetPlayersInfo _asbp_gamemode))
    (CallFunction|SetPawnDefaultRotation 2e+01 1.8e+02)
    (Variables|Default|SetPlayerIndex 1)
    (else
      (CallFunction|SetPawnDefaultRotation 2e+01 0.0)
      (Variables|Default|SetPlayerIndex -1))))

(fn ConstructionScript)