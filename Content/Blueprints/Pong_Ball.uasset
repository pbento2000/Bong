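; Pong ball pawn that launches at a random angle and, once the game starts, moves via FloatingPawnMovement, periodically easing its speed toward a base value.
; Sphere overlaps drive gameplay: walls mirror Y, while paddles re-aim by hit offset, add their speed modifier and randomly spawn power-ups, ignoring repeat hits by one player.
; Power-ups and goals report the last hitter to BP_Gamemode; goals either destroy or respawn the ball.
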(event OnComponentBeginOverlap(SphereCol)
  (params (OverlappedComponent :type Primitive%20Component%20Object%20Reference) (OtherActor :type Actor%20Object%20Reference) (OtherComp :type Primitive%20Component%20Object%20Reference) (OtherBodyIndex :type Integer) (bFromSweep :type Boolean) (SweepResult :type Hit%20Result%20Structure%20%28by%20ref%29))
  ;[1 1 1] Collision Code
  (Utilities|Casting|CastToWall_BP OtherActor
    (:then
      (Variables|Default|SetDirection (Math|Vector|MakeVector (.x (Variables|Default|GetDirection)) (* (.y (Variables|Default|GetDirection)) -1.0) (.z (Variables|Default|GetDirection))))
      (Audio|PlaySound2D "/Game/Sounds/ping_pong_8bit_plop.ping_pong_8bit_plop" 1.0 1.0 0.0 0 0))
    (:CastFailed
      (bind _aspaddle_pawn (Utilities|Casting|CastToPaddle_Pawn OtherActor)
        (:then
          (if (!= (Variables|Default|GetLastPlayerHit) (Variables|/Game/Blueprints/Paddle_Pawn.Paddle_Pawn_C|GetPlayerIndex _aspaddle_pawn))
            (bind _output_get (Variables|Default|SetLastPlayerHit (Variables|/Game/Blueprints/Paddle_Pawn.Paddle_Pawn_C|GetPlayerIndex _aspaddle_pawn)))
            (bind _returnvalue (Class|LogicandMaths|RotateBall (- (.y (Transformation|GetActorLocation _aspaddle_pawn)) (.y (Transformation|GetActorLocation))) _output_get))
            (Variables|Default|SetDirection _returnvalue)
            (Variables|Default|SetMultiplyVector (+ (Math|Conversions|ToVector(Float) (Variables|/Game/Blueprints/Paddle_Pawn.Paddle_Pawn_C|GetSpeedModifier _aspaddle_pawn)) (Variables|Default|GetMultiplyVector)))
            (CallFunction|SpawnPowerUp)
            (if (< (Variables|/Game/Blueprints/Paddle_Pawn.Paddle_Pawn_C|GetSpeedModifier _aspaddle_pawn) 0.05)
              (Audio|PlaySound2D "/Game/Sounds/ping_pong_8bit_beeep.ping_pong_8bit_beeep" 1.0 1.0 0.0 0 0)
              (else
                (Audio|PlaySound2D "/Game/Sounds/tennis-smash-100733.tennis-smash-100733" 1.0 1.0 0.0 0 0)))))
        (:CastFailed
          (bind _aspower_up (Utilities|Casting|CastToPowerUp OtherActor)
            (:then
              (bind _asbp_gamemode (Utilities|Casting|CastToBP_Gamemode (Game|GetGameMode)))
              (Default|AddPower _asbp_gamemode (Variables|Default|GetLastPlayerHit) (Variables|/Game/Blueprints/PowerUp.PowerUp_C|GetRotationModifier _aspower_up))
              (Actor|DestroyActor _aspower_up))
            (:CastFailed
              (Utilities|Casting|CastToGoal OtherActor)
              (bind _asbp_gamemode_2 (Utilities|Casting|CastToBP_Gamemode (Game|GetGameMode)))
              (bind _isgamefinished (Default|AddScore _asbp_gamemode_2 (Variables|Default|GetLastPlayerHit)))
              (if _isgamefinished
                (Actor|DestroyActor)
                (else
                  (CallFunction|RespawnBall))))))))))

(event Custom|Respawn%20ball
  ;[1 1 1] Collision Code
  (Game|SpawnActorfromClass "Pong_Ball_C" (Math|Conversions|ToTransform(Vector) "0, 0, 0") "Undefined" "MultiplyWithRoot" 0 true 0)
  (Actor|DestroyActor))

(event Custom|SpawnPowerUp
  (if (Math|Random|RandomBool)
    (Game|SpawnActorfromClass "/Game/Blueprints/PowerUp.PowerUp_C" (Math|Transform|MakeTransform (Math|Vector|MakeVector (Math|Random|RandomFloatinRange -8e+02 8e+02) (Math|Random|RandomFloatinRange -5e+02 5e+02) 0.0) "0, 0, 0" "1.000000,1.000000,1.000000") "Undefined" "MultiplyWithRoot" 0 0)))

(event Custom|SelfDestroy
  (Actor|DestroyActor))

(event EventBeginPlay
  ;[1 1 1] Sett Ball's Starting Direction
  (bind _output_get (Variables|Default|SetLastPlayerHit (Math|Integer|SelectInt 1 -1 (Math|Random|RandomBool))))
  (bind _output_get_2 (Variables|Default|SetDirection (Math|Vector|MakeVector (Math|Conversions|ToFloat(Integer) (* _output_get -1)) 0.0 0.0)))
  (Variables|Default|SetDirection (Math|Vector|RotateVectorAroundAxis _output_get_2 (Math|Random|RandomFloatinRange 0.0 6e+01) "0.000000,0.000000,1.000000")))

(event EventTick
  (params (DeltaSeconds :type Float%20%28single-precision%29))
  ;[1 1 1] Ball Movement Code
  (if (Variables|Default|GetGameStarted)
    (Class|PawnMovementComponent|AddInputVector (Variables|Default|GetFloatingPawnMovement) (* (Variables|Default|GetDirection) (Variables|Default|GetMultiplyVector)) false)
    (bind _output_get (Variables|Default|SetTimeStorer (+ (Variables|Default|GetTimeStorer) DeltaSeconds)))
    (if (and (>= _output_get (Variables|Default|GetTimeToActivate)) (Utilities|Operators|NotEqual(!=) (Variables|Default|GetMultiplyVector) "0.930000,0.930000,0.930000" 0.01))
      (Variables|Default|SetTimeStorer 0.0)
      (bind _returnvalue (Class|LogicandMaths|ReduceBallSpeedOverTime 0.93 0.15 (Variables|Default|GetMultiplyVector)))
      (bind _output_get_2 (Variables|Default|SetMultiplyVector _returnvalue))
      (Development|PrintString (Utilities|String|ToString(Vector) _output_get_2)))))

(fn ConstructionScript)